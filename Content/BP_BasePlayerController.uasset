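; Player controller that builds the on-screen HUD and player info widgets when play begins.
; It creates WBP_PlayerHUD, adds it to the viewport and registers its minimap widget with the TPBaseGameState.
; It also creates WBP_PlayerInfo, stores it on the possessed TPBaseCharacter and adds it to the viewport.
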(event `self.ReceiveBeginPlay`
  (`|ExecutionSequence`
    (:`then_0`
      (bind _returnvalue (`|CreateWidget` "/Game/UI/WBP_PlayerHUD.WBP_PlayerHUD_C"))
      (`/Engine/EditorBlueprintResources/StandardMacros.IsValid` _returnvalue
        (:`Is Valid`
          (bind _output_get (set `self.PlayerHUDWidget_0` _returnvalue))
          (`UserWidget.AddToViewport` _output_get 0)
          (bind _astpbase_game_state (cast `TPBaseGameState` (`GameplayStatics.GetGameState`)))
          (`TPBaseGameState.RegisterMap` _astpbase_game_state (`/Game/UI/WBP_PlayerHUD.WBP_MiniMapWidget` _returnvalue)))))
    (:`then_1`
      (bind _returnvalue_2 (`|CreateWidget` "/Game/UI/WBP_PlayerInfo.WBP_PlayerInfo_C"))
      (bind _astpbase_character (cast `TPBaseCharacter` (`self.K2_GetPawn`)))
      (bind _output_get_2 (set `TPBaseCharacter.PlayerInfoWidget` _returnvalue_2 _astpbase_character))
      (`UserWidget.AddToViewport` _output_get_2 0))))

(fn `UserConstructionScript`)